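; Third-person shooter character Blueprint that creates and feeds the on-screen HP UI.
; On BeginPlay it adds a WBP_ScreenUI widget for player controller 0 to the viewport, then refreshes it after a short delay.
; UpdateHPUI casts the movement component's pawn owner to TPSCharacter and passes it to the widget's UIUpdate.
; Tick, overlap and construction logic are empty.
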(event `self.ReceiveBeginPlay`
  (bind _returnvalue (`|CreateWidget` "/Game/_JaebyContent/Blueprints/WBP_ScreenUI.WBP_ScreenUI_C" (`GameplayStatics.GetPlayerController` 0)))
  (set `self.uiScreen` _returnvalue)
  (`UserWidget.AddToViewport` (`self.uiScreen`) 0)
  (`KismetSystemLibrary.Delay` 0.05)
  (`self.UpdateHPUI`))

(fn `UpdateHPUI`
  (bind _astpscharacter (cast `TPSCharacter` (`PawnMovementComponent.GetPawnOwner` (`self.CharacterMovement`))))
  (`/Game/_JaebyContent/Blueprints/WBP_ScreenUI.UIUpdate` (`self.uiScreen`) _astpscharacter))

(fn `UserConstructionScript`)