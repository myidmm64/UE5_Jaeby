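; An enemy spawner for the TPS game that keeps creating BP_Enemy actors at randomized intervals.
; On BeginPlay it caches the first BP_TPSCharacter as the target, and Tick accumulates a timer that triggers SpawnEnemy and re-rolls the next delay.
; Each enemy spawns at a random XY offset from the world origin, not the spawner, at a set height, then receives the target and an effectively fixed speed through InitEnemy.
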(event `self.ReceiveBeginPlay`
  (bind _outactors (`GameplayStatics.GetAllActorsOfClass` "/Game/TPSContent/Blueprints/BP_TPSCharacter.BP_TPSCharacter_C"))
  (set `self.playerTarget` (`|GetArrayItem` _outactors)))

(event `self.ReceiveTick`
  (params (DeltaSeconds :type "Float (single-precision)"))
  (bind _output_get (set `self.Timer` (+ DeltaSeconds (`self.Timer`))))
  (if (>= _output_get (`self.SpawnTime`))
    (`self.SpawnEnemy`)
    (set `self.Timer` 0.0)
    (set `self.SpawnTime` (`KismetMathLibrary.RandomFloatInRange` (`self.MinSpawnTime`) (`self.MaxSpawnTime`)))))

(event `self.ReceiveActorBeginOverlap`
  (params (OtherActor :type "Actor Object Reference")))

(fn `SpawnEnemy`
  (bind _returnvalue (`|SpawnActorFromClass` "/Game/TPSContent/Blueprints/BP_Enemy.BP_Enemy_C" (`KismetMathLibrary.MakeTransform` (`KismetMathLibrary.MakeVector` (.x (* (`KismetMathLibrary.RandomUnitVector`) (`KismetMathLibrary.RandomFloatInRange` 0.0 1000.0))) (.y (* (`KismetMathLibrary.RandomUnitVector`) (`KismetMathLibrary.RandomFloatInRange` 0.0 1000.0))) (`self.zLocation`))) "Undefined" "OverrideRootScale" null null))
  (`Enemy.InitEnemy` _returnvalue (`self.playerTarget`) (`KismetMathLibrary.RandomFloatInRange` 100.0 100.0)))

(fn `UserConstructionScript`)